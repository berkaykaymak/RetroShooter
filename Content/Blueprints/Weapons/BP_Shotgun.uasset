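; Shotgun weapon Blueprint that overrides shooting on a weapon base with a Paper2D flipbook sprite.
; ShootWeapon checks for ammo, then passes a DoOnce gate to decrease ammo, fire and switch to the fire flipbook.
; After a delay equal to that flipbook's length, it restores the idle flipbook and resets the gate, so the animation length sets the fire rate.
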(event Custom|ResetFire
  (bind _weaponbaseflipbook (Variables|Default|GetWeaponBaseFlipBook))
  (Utilities|FlowControl|DoOnce false) ; enters at Reset
)

(event EventBeginPlay
  (|CallParentFunction) ; This node is disabled and will not be called.\nDrag off pins to build functionality.
)

(event Collision|EventActorBeginOverlap
  (params (OtherActor :type Actor%20Object%20Reference))
  (|CallParentFunction OtherActor) ; This node is disabled and will not be called.\nDrag off pins to build functionality.
)

(event EventTick
  (params (DeltaSeconds :type Float%20%28single-precision%29))
  (|CallParentFunction DeltaSeconds) ; This node is disabled and will not be called.\nDrag off pins to build functionality.
)

(event EventShootWeapon
  (bind _weaponbaseflipbook (Variables|Default|GetWeaponBaseFlipBook))
  (bind _hasammo (CallFunction|HasEnoughAmmo))
  (if _hasammo
    (Utilities|FlowControl|DoOnce false
      (:Completed
        (CallFunction|DecreaseAmmo)
        (CallFunction|FireWeapon)
        (Sprite|SetFlipbook _weaponbaseflipbook "/Game/Sprites/Weapons/Shotgun/FB_ShotgunFire.FB_ShotgunFire")
        (Utilities|FlowControl|Delay (Class|PaperFlipbookComponent|GetFlipbookLength _weaponbaseflipbook))
        (Sprite|SetFlipbook (Variables|Default|GetWeaponBaseFlipBook) "/Game/Sprites/Weapons/Shotgun/FB_ShotgunIdle.FB_ShotgunIdle")
        (CallFunction|ResetFire)))))

(fn ConstructionScript
  (|CallParentFunction))