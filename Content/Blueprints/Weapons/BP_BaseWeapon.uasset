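; BP_BaseWeapon is a base weapon Blueprint for the first-person character, with empty ShootWeapon and StopShooting events.
; It caches the player character and controller on BeginPlay.
; FireWeapon line-traces forward from the LineTrace component, with debug drawing, and applies WeaponDamage to the hit actor.
; HasEnoughAmmo and DecreaseAmmo switch on AmmoType to check or decrement the character's ammo pools, with DecreaseAmmo also updating the HUD.
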(event Custom|ShootWeapon)

(event Custom|StopShooting)

(event Custom|DecreaseAmmo
  (bind _playercontrollerref (Variables|Default|GetPlayerControllerRef))
  (bind _hudref (Variables|/Game/FirstPerson/Blueprints/BP_FirstPersonPlayerController.BP_FirstPersonPlayerController_C|GetHUDRef _playercontrollerref))
  (switch Utilities|FlowControl|Switch|SwitchonEnum_Ammo (Variables|Default|GetAmmoType)
    (:NewEnumerator0
      (Math|Integer|DecrementInt (Variables|/Game/FirstPerson/Blueprints/BP_FirstPersonCharacter.BP_FirstPersonCharacter_C|GetBullet (Variables|Default|GetPlayerCharacterRef))
        (:%20%20
          (Default|UpdateBullet _hudref))))
    (:NewEnumerator1
      (Math|Integer|DecrementInt (Variables|/Game/FirstPerson/Blueprints/BP_FirstPersonCharacter.BP_FirstPersonCharacter_C|GetShell (Variables|Default|GetPlayerCharacterRef))
        (:%20%20
          (Default|UpdateShell _hudref))))
    (:NewEnumerator2
      (Math|Integer|DecrementInt (Variables|/Game/FirstPerson/Blueprints/BP_FirstPersonCharacter.BP_FirstPersonCharacter_C|GetRocket (Variables|Default|GetPlayerCharacterRef))
        (:%20%20
          (Default|UpdateRocket _hudref))))
    (:NewEnumerator3
      (Math|Integer|DecrementInt (Variables|/Game/FirstPerson/Blueprints/BP_FirstPersonCharacter.BP_FirstPersonCharacter_C|GetCell (Variables|Default|GetPlayerCharacterRef))
        (:%20%20
          (Default|UpdateCell _hudref))))))

(event EventBeginPlay
  (bind _asbp_first_person_character (Utilities|Casting|CastToBP_FirstPersonCharacter (Game|GetPlayerCharacter 0)))
  (Variables|Default|SetPlayerCharacterRef _asbp_first_person_character)
  (bind _asbp_first_person_player_controller (Utilities|Casting|CastToBP_FirstPersonPlayerController (Game|GetPlayerController 0)))
  (Variables|Default|SetPlayerControllerRef _asbp_first_person_player_controller))

(fn ConstructionScript)

(fn FireWeapon
  (bind _linetrace (Variables|Default|GetLineTrace))
  (bind _returnvalue (Transformation|GetWorldLocation _linetrace))
  (bind (_outhit _returnvalue_2) (Collision|LineTraceForObjects _returnvalue (+ _returnvalue (* (Math|Vector|GetForwardVector (Transformation|GetWorldRotation (Variables|Default|GetLineTrace))) (Variables|Default|GetLineTraceDistance))) (Utilities|Array|MakeArray "ObjectTypeQuery1" "ObjectTypeQuery2" "ObjectTypeQuery3") false (Utilities|Array|MakeArray self (Game|GetPlayerCharacter 0)) "ForDuration"))
  (if _returnvalue_2
    (Game|Damage|ApplyDamage (.HitActor (Collision|BreakHitResult _outhit)) (Variables|Default|GetWeaponDamage) 0 0)))

(fn HasEnoughAmmo
  (switch Utilities|FlowControl|Switch|SwitchonEnum_Ammo (Variables|Default|GetAmmoType)
    (:NewEnumerator0
      (if (> (Variables|/Game/FirstPerson/Blueprints/BP_FirstPersonCharacter.BP_FirstPersonCharacter_C|GetBullet (Variables|Default|GetPlayerCharacterRef)) 0)
        (return true)
        (else
          (return false))))
    (:NewEnumerator1
      (if (> (Variables|/Game/FirstPerson/Blueprints/BP_FirstPersonCharacter.BP_FirstPersonCharacter_C|GetShell (Variables|Default|GetPlayerCharacterRef)) 0)
        (return true)
        (else
          (return false))))
    (:NewEnumerator2
      (if (> (Variables|/Game/FirstPerson/Blueprints/BP_FirstPersonCharacter.BP_FirstPersonCharacter_C|GetRocket (Variables|Default|GetPlayerCharacterRef)) 0)
        (return true)
        (else
          (return false))))
    (:NewEnumerator3
      (if (> (Variables|/Game/FirstPerson/Blueprints/BP_FirstPersonCharacter.BP_FirstPersonCharacter_C|GetCell (Variables|Default|GetPlayerCharacterRef)) 0)
        (return true)
        (else
          (return false))))))